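; BP_Vector is a test actor that compares three ways of offsetting its location with vector math.
; BeginPlay runs only Case3, which moves it 100 units along the normalized 2D forward vector of a 45-degree yaw.
; The unused Case2 does the same with the actor's own rotation.
; The unused Case1 adds a fixed XY offset and prints the XY length of the resulting position.
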(event `Case3`
  ;[0.65 0.2601 1] Case3
  (`self.K2_SetActorLocation` (+ (`self.K2_GetActorLocation`) (* (`KismetMathLibrary.Vector_Normal2D` (`KismetMathLibrary.GetForwardVector` (`KismetMathLibrary.MakeRotator` 0.0 0.0 45.0))) 100.0))))

(event `Case2`
  ;[0.2271 0.5191 1] Case2
  (`self.K2_SetActorLocation` (+ (`self.K2_GetActorLocation`) (* (`KismetMathLibrary.Vector_Normal2D` (`KismetMathLibrary.GetForwardVector` (`self.K2_GetActorRotation`))) 100.0))))

(event `self.ReceiveBeginPlay`
  (`self.Case3`))

(event `Case1`
  (bind _returnvalue (+ (`self.K2_GetActorLocation`) (`KismetMathLibrary.MakeVector` 100.0 100.0)))
  ;[0.3895 1 0.3336] Case1
  (`self.K2_SetActorLocation` _returnvalue)
  (`KismetSystemLibrary.PrintString` (`KismetStringLibrary.Conv_DoubleToString` (`KismetMathLibrary.VSizeXY` _returnvalue)) true true (struct :`G` 0.66 :`B` 1.0 :`A` 1.0) 5.0))

(fn `UserConstructionScript`)