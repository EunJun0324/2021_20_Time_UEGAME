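; BP_Hit is a basic debug actor that reports collision and overlap events on its Box component.
; It binds the Box's hit, begin overlap and end overlap events, each printing a label with the other actor's and component's display names.
; The construction script is empty, so all behavior lives in these three event handlers.
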(event `self.Box.OnComponentHit`
  (params (HitComponent :type "PrimitiveComponent Object Reference") (OtherActor :type "Actor Object Reference") (OtherComp :type "PrimitiveComponent Object Reference") (NormalImpulse :type "Vector Structure") (Hit :type "HitResult Structure (by ref)"))
  (`KismetSystemLibrary.PrintString` (`KismetStringLibrary.Concat_StrStr` "Hit : " (`KismetSystemLibrary.GetDisplayName` OtherActor) (`KismetSystemLibrary.GetDisplayName` OtherComp))))

(event `self.Box.OnComponentBeginOverlap`
  (params (OverlappedComponent :type "PrimitiveComponent Object Reference") (OtherActor :type "Actor Object Reference") (OtherComp :type "PrimitiveComponent Object Reference") (OtherBodyIndex :type Integer) (bFromSweep :type Boolean) (SweepResult :type "HitResult Structure (by ref)"))
  (`KismetSystemLibrary.PrintString` (`KismetStringLibrary.Concat_StrStr` "Begin : " (`KismetSystemLibrary.GetDisplayName` OtherActor) (`KismetSystemLibrary.GetDisplayName` OtherComp))))

(event `self.Box.OnComponentEndOverlap`
  (params (OverlappedComponent :type "PrimitiveComponent Object Reference") (OtherActor :type "Actor Object Reference") (OtherComp :type "PrimitiveComponent Object Reference") (OtherBodyIndex :type Integer))
  (`KismetSystemLibrary.PrintString` (`KismetStringLibrary.Concat_StrStr` "End  : " (`KismetSystemLibrary.GetDisplayName` OtherActor) (`KismetSystemLibrary.GetDisplayName` OtherComp))))

(fn `UserConstructionScript`)