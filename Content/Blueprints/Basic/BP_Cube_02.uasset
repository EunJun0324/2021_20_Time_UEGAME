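; BP_Cube_02 is a basic Blueprint that exercises variable math and on-screen debug printing.
; On BeginPlay it prints the sum of variables A and B for ten seconds.
; Each Tick it adds DeltaSeconds to C, a running time counter, and prints the value in cyan.
; The construction script is empty.
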(event `self.ReceiveBeginPlay`
  (`KismetSystemLibrary.PrintString` (`KismetStringLibrary.Conv_IntToString` (+ (`self.A`) (`self.B`))) true true (struct :`G` 0.66 :`B` 1.0 :`A` 1.0) 10.0))

(event `self.ReceiveTick`
  (params (DeltaSeconds :type "Float (single-precision)"))
  (bind _output_get (set `self.C` (+ DeltaSeconds (`self.C`))))
  (`KismetSystemLibrary.PrintString` (`KismetStringLibrary.Conv_DoubleToString` _output_get) true true (struct :`G` 0.89433 :`B` 1.0 :`A` 1.0)))

(fn `UserConstructionScript`)