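; Anim notify state "Collision" that switches on the player's one-handed weapon collision for a window within an animation.
; On begin it casts the mesh owner to BP_Player and sets the OneHand capsule to Query and Physics; on end it sets it back to No Collision.
; Owners that are not BP_Player are ignored.
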(fn `GetNotifyName`
  (returns (ReturnValue :type String))
  (return "Collision"))

(fn `Received_NotifyBegin`
  (params (MeshComp :type "SkeletalMeshComponent Object Reference") (Animation :type "AnimSequenceBase Object Reference") (TotalDuration :type "Float (double-precision)"))
  (returns (ReturnValue :type Boolean))
  (bind _asbp_player (cast `/Game/Blueprints/Player/BP_Player` (`ActorComponent.GetOwner` MeshComp)))
  (`PrimitiveComponent.SetCollisionEnabled` (`/Game/Blueprints/Weapons/BP_Sword.Capsule` (`/Game/Blueprints/Player/BP_Player.OneHand` _asbp_player)) "QueryAndPhysics")
  (return false))

(fn `Received_NotifyEnd`
  (params (MeshComp :type "SkeletalMeshComponent Object Reference") (Animation :type "AnimSequenceBase Object Reference"))
  (returns (ReturnValue :type Boolean))
  (bind _asbp_player (cast `/Game/Blueprints/Player/BP_Player` (`ActorComponent.GetOwner` MeshComp)))
  (`PrimitiveComponent.SetCollisionEnabled` (`/Game/Blueprints/Weapons/BP_Sword.Capsule` (`/Game/Blueprints/Player/BP_Player.OneHand` _asbp_player)) "NoCollision")
  (return false))