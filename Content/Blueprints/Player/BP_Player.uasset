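; Player character with camera-relative movement and one-handed sword combat, including equip and sheath, a roll or backstep dodge, and combo attacks.
; A sword spawned at BeginPlay moves between holster and hand sockets; drawing it switches to controller-facing rotation and turns Jump into a dodge.
; State flags lock movement during actions until End events clear them.
; Attack presses during a combo window queue the next montage, played by NextAction.
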(fn `AttachWeapon`
  (params (inActor :type "Actor Object Reference") (inParent :type "SkeletalMeshComponent Object Reference") (inSocketName :type Name))
  (`self.K2_AttachToComponent` inActor inParent inSocketName "KeepRelative" "KeepRelative" "KeepRelative" true))

(fn `UserConstructionScript`)