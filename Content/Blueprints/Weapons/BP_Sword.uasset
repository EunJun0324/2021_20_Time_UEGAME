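; BP_Sword is a melee weapon that damages characters it strikes on behalf of its owning player.
; Its capsule hitbox starts with collision disabled on BeginPlay, and nothing in this file turns it back on.
; On overlap, any Character other than the owner takes fixed damage, credited to the owner's controller, provided the owner is a BP_Player.
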(event `self.ReceiveBeginPlay`
  (`PrimitiveComponent.SetCollisionEnabled` (`self.Capsule`) "NoCollision"))

(event `self.Capsule.OnComponentBeginOverlap`
  (params (OverlappedComponent :type "PrimitiveComponent Object Reference") (OtherActor :type "Actor Object Reference") (OtherComp :type "PrimitiveComponent Object Reference") (OtherBodyIndex :type Integer) (bFromSweep :type Boolean) (SweepResult :type "HitResult Structure (by ref)"))
  (if (!= OtherActor (`self.GetOwner`))
    (bind _ascharacter (cast `Character` OtherActor))
    (bind _asbp_player (cast `/Game/Blueprints/Player/BP_Player` (`self.GetOwner`)))
    (`GameplayStatics.ApplyDamage` _ascharacter 20.0 (`Pawn.GetController` _asbp_player) self)))

(fn `UserConstructionScript`)